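; BP_LevelSelection is a level portal that opens the level named by LevelName after a countdown inside its trigger box.
; Beginning overlap starts a looping one-second timer that decrements BoxTime, prints the remaining seconds and travels at zero.
; Ending overlap before travel clears the timer and prints a cancellation, without resetting BoxTime.
; The construction script fills its two text components from the World and Description variables.
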(event OnComponentBeginOverlap(Box)
  (params (OverlappedComponent :type Primitive%20Component%20Object%20Reference) (OtherActor :type Actor%20Object%20Reference) (OtherComp :type Primitive%20Component%20Object%20Reference) (OtherBodyIndex :type Integer) (bFromSweep :type Boolean) (SweepResult :type Hit%20Result%20Structure%20%28by%20ref%29))
  ;[0 1 1] Overlapped box
  ;[1 1 1] Set countdown timer
  (if (not (Utilities|Time|IsValidTimerHandle (Variables|Default|GetEnteredBoxTimer)))
    (bind _returnvalue (Utilities|Time|SetTimerbyEvent (delegate Custom|BoxTimerTick) 1.0 true))
    (Variables|Default|SetEnteredBoxTimer _returnvalue)))

(event OnComponentEndOverlap(Box)
  (params (OverlappedComponent :type Primitive%20Component%20Object%20Reference) (OtherActor :type Actor%20Object%20Reference) (OtherComp :type Primitive%20Component%20Object%20Reference) (OtherBodyIndex :type Integer))
  ;[1 0 0] End overlap, clear timer
  (if (not (Variables|Default|GetTravelling))
    (Utilities|Time|ClearandInvalidateTimerbyHandle (Variables|Default|GetEnteredBoxTimer))
    (Development|PrintString "TRANSITION CANCELLED!")))

(event Custom|BoxTimerTick
  (bind _boxtime (Variables|Default|GetBoxTime))
  ;[1 1 1] Countdown on timer
  (if (== _boxtime 0)
    ;[0 1 0] Open level
    (Variables|Default|SetTravelling true)
    (Game|OpenLevel(byName) (Variables|Defaults|GetLevelName))
    (else
      (Math|Integer|DecrementInt _boxtime
        (:%20%20
          (Development|PrintString (Utilities|String|Append "TRAVELLING TO LEVEL IN: " (Utilities|String|ToString(Integer) _boxtime) " (seconds)")))))))

(fn ConstructionScript
  (Rendering|Components|TextRender|SetText (Variables|References|GetExampleWorldText) (Variables|Defaults|GetWorld))
  (Rendering|Components|TextRender|SetText (Variables|Default|GetDescriptionText) (Variables|Defaults|GetDescription)))